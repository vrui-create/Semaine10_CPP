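; BP_Cible is a target actor in the VATS folder with a widget that turns toward the player camera every tick.
; On BeginPlay it passes itself to its UI_Cible widget as a reference.
; A sphere overlap shows the widget when the player character enters and hides it on exit.
; CE_Play_Scale alternately plays and reverses a timeline scaling the whole actor, gated by a DoOnce.
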(event `self.ReceiveBeginPlay`
  (bind _asui_cible (cast `/Game/VATS/Cibler/UI_Cible` (`WidgetComponent.GetWidget` (`self.Widget`))))
  (set `/Game/VATS/Cibler/UI_Cible.Ref BP Cible` self _asui_cible))

(event `self.ReceiveTick`
  (params (DeltaSeconds :type "Float (single-precision)"))
  (`self.F_UI_Look_Player`))

(event `CE_Play_Scale`
  ; Ce code permet de progressivement changer la taille Global de l'actor
  (`/Engine/EditorBlueprintResources/StandardMacros.DoOnce` false :!label _label
    (:`Completed`
      (`/Engine/EditorBlueprintResources/StandardMacros.FlipFlop`
        (:`A`
          (bind (_direction _vector_scale) (`Timeline|Timeline` :!via `PlayFromStart` :!label _label_2)
            (:`Update`
              (`self.SetActorScale3D` (`KismetMathLibrary.Conv_DoubleToVector` (* _vector_scale 1.0))))
            (:`Finished`
              (goto _label :!via `Reset`))))
        (:`B`
          (goto _label_2 :!via `ReverseFromEnd`))))))

(event `self.Sphere.OnComponentBeginOverlap`
  (params (OverlappedComponent :type "PrimitiveComponent Object Reference") (OtherActor :type "Actor Object Reference") (OtherComp :type "PrimitiveComponent Object Reference") (OtherBodyIndex :type Integer) (bFromSweep :type Boolean) (SweepResult :type "HitResult Structure (by ref)"))
  ; Ce code permet de cacher UI ou Widget quand le joueur s'éloigne de cette objet, et inversement si il s'approche, la il apparait
  (if (== OtherActor (`GameplayStatics.GetPlayerCharacter` 0))
    (`SceneComponent.SetHiddenInGame` (`self.Widget`) false false)))

(event `self.Sphere.OnComponentEndOverlap`
  (params (OverlappedComponent :type "PrimitiveComponent Object Reference") (OtherActor :type "Actor Object Reference") (OtherComp :type "PrimitiveComponent Object Reference") (OtherBodyIndex :type Integer))
  ; Ce code permet de cacher UI ou Widget quand le joueur s'éloigne de cette objet, et inversement si il s'approche, la il apparait
  (if (== (`GameplayStatics.GetPlayerCharacter` 0) OtherActor)
    (`SceneComponent.SetHiddenInGame` (`self.Widget`) true false)))

(fn `F_UI_Look_Player`
  (bind _returnvalue (`GameplayStatics.GetPlayerCameraManager` 0))
  (`/Engine/EditorBlueprintResources/StandardMacros.IsValid` _returnvalue
    (:`Is Valid`
      (`SceneComponent.K2_SetRelativeRotation` (`self.Widget`) (`KismetMathLibrary.FindLookAtRotation` (`self.K2_GetActorLocation`) (`self.K2_GetActorLocation` _returnvalue)) false false))))

(fn `UserConstructionScript`)