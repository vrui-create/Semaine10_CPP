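; Player character that handles Enhanced Input for camera-relative movement, jumping with sound, camera control and target interaction.
; BeginPlay adds the input mapping context and activates the main camera, while look input rotates the spring arm and movement turns the mesh.
; The aim input toggles between the main and aiming cameras on the same character.
; Interaction line-traces from the aiming camera, with persistent debug drawing, and triggers a scale event on BP_Cible targets.
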(event `self.ReceiveBeginPlay`
  (`self.F_Setup_Player`))

(event `EnhancedInput|/Game/VATS/Player_Charactere/Input_System/IA_Moving`
  (params (ActionValue :type "Vector2D Structure") (ElapsedSeconds :type "Float (double-precision)") (TriggeredSeconds :type "Float (double-precision)") (InputAction :type "InputAction Object Reference" :default "/Game/VATS/Player_Charactere/Input_System/IA_Moving.IA_Moving"))
  (bind (_returnvalue_roll _returnvalue_pitch _returnvalue_yaw) (`KismetMathLibrary.BreakRotator` (`KismetMathLibrary.MakeRotator` ActionValue_X ActionValue_Y)))
  (bind (_rigth__vector _forward_vector) (`self.M_Setup_Player`))
  (bind (_returnvalue_roll_2 _returnvalue_pitch_2 _returnvalue_yaw_2) (`KismetMathLibrary.BreakRotator` (`SceneComponent.K2_GetComponentRotation` (`self.Mesh`))))
  (:`Triggered`
    (`self.AddMovementInput` _rigth__vector ActionValue_X true)
    (`self.AddMovementInput` _forward_vector ActionValue_Y true)
    (`SceneComponent.K2_SetRelativeRotation` (`self.Mesh`) (`KismetMathLibrary.MakeRotator` 0.0 0.0 (`KismetMathLibrary.Lerp` _returnvalue_yaw _returnvalue_yaw_2 0.5)) false false)))

(event `EnhancedInput|/Game/VATS/Player_Charactere/Input_System/IA_Jumping`
  (params (ActionValue :type Boolean) (ElapsedSeconds :type "Float (double-precision)") (TriggeredSeconds :type "Float (double-precision)") (InputAction :type "InputAction Object Reference" :default "/Game/VATS/Player_Charactere/Input_System/IA_Jumping.IA_Jumping"))
  ; IA jumping setup from player
  (:`Triggered`
    (if (not (`NavMovementComponent.IsFalling` (`self.CharacterMovement`)))
      (`self.Jump`)
      (`GameplayStatics.PlaySoundAtLocation` "/Game/VATS/Cibler/SC_Jumpt.SC_Jumpt" (`self.K2_GetActorLocation`) (struct) 1.0 1.0 0.0 null null null null)))
  (:`Completed`
    (`self.StopJumping`)))

(event `EnhancedInput|/Game/VATS/Player_Charactere/Input_System/IA_Camering`
  (params (ActionValue :type "Vector2D Structure") (ElapsedSeconds :type "Float (double-precision)") (TriggeredSeconds :type "Float (double-precision)") (InputAction :type "InputAction Object Reference" :default "/Game/VATS/Player_Charactere/Input_System/IA_Camering.IA_Camering"))
  ; Controlle la camera
  (:`Triggered`
    (`self.M_Move_Camera` ActionValue_X ActionValue_Y)))

(event `EnhancedInput|/Game/VATS/Player_Charactere/Input_System/IA_Interaction_Objet`
  (params (ActionValue :type Boolean) (ElapsedSeconds :type "Float (double-precision)") (TriggeredSeconds :type "Float (double-precision)") (InputAction :type "InputAction Object Reference" :default "/Game/VATS/Player_Charactere/Input_System/IA_Interaction_Objet.IA_Interaction_Objet"))
  (bind (`_point_de_départ_du_line_trace_` _point_de_fin_du_linetrace) (`self.M_Line_Trace` (`SceneComponent.K2_GetComponentLocation` (`self.Viseur_Camera`)) 500.0))
  ; Interaction objet
  (:`Started`
    (bind (_outhit _returnvalue) (`KismetSystemLibrary.LineTraceSingle` :`Start` `_point_de_départ_du_line_trace_` :`End` _point_de_fin_du_linetrace :`TraceChannel` "TraceTypeQuery1" :`DrawDebugType` "Persistent"))
    (bind (_bblockinghit _binitialoverlap _time _distance _location _impactpoint _normal _impactnormal _physmat _hitactor) (`GameplayStatics.BreakHitResult` _outhit))
    (bind _asbp_cible (cast `/Game/VATS/BP_Cible` _hitactor :!pure true))
    (if (and _returnvalue (== _hitactor _asbp_cible))
      (set `self.As BP Cible` _asbp_cible)
      (`/Game/VATS/BP_Cible.CE_Play_Scale` (`self.As BP Cible`)))))

(event `EnhancedInput|/Game/VATS/Player_Charactere/Input_System/IA_Viseur`
  (params (ActionValue :type Boolean) (ElapsedSeconds :type "Float (double-precision)") (TriggeredSeconds :type "Float (double-precision)") (InputAction :type "InputAction Object Reference" :default "/Game/VATS/Player_Charactere/Input_System/IA_Viseur.IA_Viseur"))
  (bind _viseur_camera (`self.Viseur_Camera`))
  (bind _camera (`self.Camera`))
  ; Ce Code permet d'intervertire entre deux camera dans le même player character.
  (:`Started`
    (if (`ActorComponent.IsActive` (`self.Camera`))
      (`ActorComponent.SetActive` _camera false false)
      (`ActorComponent.SetActive` _viseur_camera true false)
      (else
        (`ActorComponent.SetActive` _camera true false)
        (`ActorComponent.SetActive` _viseur_camera false false)))))

(fn `F_Setup_Player`
  (bind _returnvalue (pcsubsystem `EnhancedInputLocalPlayerSubsystem` (`GameplayStatics.GetPlayerController` 0)))
  (`/Engine/EditorBlueprintResources/StandardMacros.IsValid` _returnvalue
    (:`Is Valid`
      (`EnhancedInputSubsystemInterface.AddMappingContext` _returnvalue "/Game/VATS/Player_Charactere/Input_System/Liste_Input_Action.Liste_Input_Action" 0 (struct))
      (cast `/Game/VATS/MultiJoueur/GI_Save_Temporaire` (`GameplayStatics.GetGameInstance`))
      (`ActorComponent.SetActive` (`self.Viseur_Camera`) false false)
      (`ActorComponent.SetActive` (`self.Camera`) true false))))

(fn `UserConstructionScript`)