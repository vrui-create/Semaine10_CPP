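; Player character Blueprint for the VATS project, handling movement, jumping and camera through Enhanced Input.
; BeginPlay adds the input mapping context via the PlayerController_Vats subsystem.
; A macro supplies camera-yaw forward and right vectors for movement, though rightward input is a constant 1.0 rather than the action's X.
; Camera input adds directly to SpringArm pitch and yaw without clamping, and the legacy axis events are empty.
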(event `self.ReceiveBeginPlay`
  (`self.F_Setup_Player`))

(event `InputAxis|MovePlayer_ZS`
  (params (AxisValue :type "Float (single-precision)")))

(event `EnhancedInput|/Game/VATS/Player_Charactere/Input_System/IA_Moving`
  (params (ActionValue :type "Vector2D Structure") (ElapsedSeconds :type "Float (double-precision)") (TriggeredSeconds :type "Float (double-precision)") (InputAction :type "InputAction Object Reference" :default "/Game/VATS/Player_Charactere/Input_System/IA_Moving.IA_Moving"))
  (bind (_forward_vector _rigth__vector) (`self.M_Setup_Player`))
  (:`Triggered`
    (`self.AddMovementInput` _forward_vector ActionValue_Y)
    (`self.AddMovementInput` _rigth__vector)))

(event `InputAxis|MovePlayer_DQ`
  (params (AxisValue :type "Float (single-precision)")))

(event `EnhancedInput|/Game/VATS/Player_Charactere/Input_System/IA_Jumping`
  (params (ActionValue :type Boolean) (ElapsedSeconds :type "Float (double-precision)") (TriggeredSeconds :type "Float (double-precision)") (InputAction :type "InputAction Object Reference" :default "/Game/VATS/Player_Charactere/Input_System/IA_Jumping.IA_Jumping"))
  ; IA jumping setup from player
  (:`Triggered`
    (`self.Jump`))
  (:`Completed`
    (`self.StopJumping`)))

(event `EnhancedInput|/Game/VATS/Player_Charactere/Input_System/IA_Camering`
  (params (ActionValue :type "Vector2D Structure") (ElapsedSeconds :type "Float (double-precision)") (TriggeredSeconds :type "Float (double-precision)") (InputAction :type "InputAction Object Reference" :default "/Game/VATS/Player_Charactere/Input_System/IA_Camering.IA_Camering"))
  (bind (_relativerotation_roll _relativerotation_pitch _relativerotation_yaw) (`KismetMathLibrary.BreakRotator` (`SceneComponent.RelativeRotation` (`self.SpringArm`))))
  (:`Triggered`
    (`SceneComponent.K2_SetRelativeRotation` (`self.SpringArm`) (`KismetMathLibrary.MakeRotator` 0.0 (+ ActionValue_Y _relativerotation_pitch) (+ ActionValue_X _relativerotation_yaw)) false false)))

(fn `F_Setup_Player`
  (bind _asplayer_controller_vats (cast `/Game/VATS/Player_Charactere/PlayerController_Vats` (`GameplayStatics.GetPlayerController` 0)))
  (bind _returnvalue (pcsubsystem `EnhancedInputLocalPlayerSubsystem` _asplayer_controller_vats))
  (`/Engine/EditorBlueprintResources/StandardMacros.IsValid` _returnvalue
    (:`Is Valid`
      (`EnhancedInputSubsystemInterface.AddMappingContext` _returnvalue "/Game/VATS/Player_Charactere/Input_System/Liste_Input_Action.Liste_Input_Action" 0 (struct)))))

(fn `UserConstructionScript`)